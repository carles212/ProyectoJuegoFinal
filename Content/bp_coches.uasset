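; Car NPC actor (bp_coches) that makes a single straight pass along the world X axis, then destroys itself.
; On BeginPlay it stays hidden for a random whole-second delay, staggering its appearance, then shows itself and plays the MovimientoNPCs timeline.
; The timeline track sets absolute X, negated when Direccion is false to mirror travel, while Y and Z are preserved.
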(event EventBeginPlay
  (bind _returnvalue (Transformation|GetActorLocation))
  ;[1 1 1] Movimiento del NPC
  (Rendering|SetActorHiddenInGame true)
  (Utilities|FlowControl|Delay (Math|Conversions|ToFloat(Integer) (Math|Random|RandomIntegerinRange 0 12)))
  (Rendering|SetActorHiddenInGame false)
  (bind _新規track_1 (Timeline|movimientoNPCs Play)
    (:Update
      (if (Variables|Default|Getdireccion)
        (Transformation|SetActorLocation (Math|Vector|MakeVector _新規track_1 (.y _returnvalue) (.z _returnvalue)) false false)
        (else
          (Transformation|SetActorLocation (Math|Vector|MakeVector (* _新規track_1 -1.0) (.y _returnvalue) (.z _returnvalue)) false false))))
    (:Finished
      (Actor|DestroyActor))))

(fn ConstructionScript)