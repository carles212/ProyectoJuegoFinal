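; Ferris wheel actor that spins continuously from the moment play begins.
; A Timeline started on BeginPlay drives the main wheel mesh's relative roll through a scaled full turn, then replays from the start after a brief delay.
; Each update also resets the twelve other wheel components to zero world rotation, so they stay upright as the wheel turns.
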(event EventBeginPlay
  (bind _newtrack_0 (Timeline|Timeline Play)
    (:Update
      (Transformation|SetRelativeRotation (Variables|Default|GetnoriaGenteNoMuere_carnival_ferris_wheel) (Math|Rotator|MakeRotator (* _newtrack_0 3.6e+02) 0.0 0.0) false false)
      (Transformation|SetWorldRotation (Variables|Default|GetnoriaGenteNoMuere_carnival_ferris_wheel_004) "0, 0, 0" false false))
    (:Finished
      (Utilities|FlowControl|Delay 0.02)
      (Timeline|Timeline PlayFromStart))))

(fn ConstructionScript)