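; Walking NPC actor that gets a random character look and dialogue line on BeginPlay.
; Outside the tutorial, a timeline moves it along X toward the player's starting side, then destroys it when finished.
; Overlapping the player with its box stops the timeline, leaving the NPC in place.
; One of three mesh and looping walk animation pairs is picked, and one random phrase fills both dialogue widgets.
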(event OnComponentBeginOverlap(Box)
  (params (OverlappedComponent :type Primitive%20Component%20Object%20Reference) (OtherActor :type Actor%20Object%20Reference) (OtherComp :type Primitive%20Component%20Object%20Reference) (OtherBodyIndex :type Integer) (bFromSweep :type Boolean) (SweepResult :type Hit%20Result%20Structure%20%28by%20ref%29))
  (bind _returnvalue (Transformation|GetActorLocation))
  (bind _posicioninicial (Variables|Default|GetposicionInicial))
  ;[1 1 1] Movimiento del NPC
  (Utilities|Casting|CastToBP_ThirdPersonCharacter OtherActor)
  (bind _新規track_1 (Timeline|movimientoNPCs Stop)
    (:Update
      (if (Variables|Default|GetdireccionNPCs)
        (Transformation|SetActorLocation (Math|Vector|MakeVector (+ (.x _posicioninicial) _新規track_1) (.y _returnvalue) (.z _returnvalue)) false false)
        (else
          (Transformation|SetActorLocation (Math|Vector|MakeVector (- (.x _posicioninicial) _新規track_1) (.y _returnvalue) (.z _returnvalue)) false false))))
    (:Finished
      (Actor|DestroyActor))))

(event Custom|Movimiento
  (bind _returnvalue (Transformation|GetActorLocation))
  (bind _posicioninicial (Variables|Default|GetposicionInicial))
  ;[1 1 1] Movimiento del NPC
  (bind _新規track_1 (Timeline|movimientoNPCs Play)
    (:Update
      (if (Variables|Default|GetdireccionNPCs)
        (Transformation|SetActorLocation (Math|Vector|MakeVector (+ (.x _posicioninicial) _新規track_1) (.y _returnvalue) (.z _returnvalue)) false false)
        (else
          (Transformation|SetActorLocation (Math|Vector|MakeVector (- (.x _posicioninicial) _新規track_1) (.y _returnvalue) (.z _returnvalue)) false false))))
    (:Finished
      (Actor|DestroyActor))))

(event EventBeginPlay
  (bind _skeletalmesh (Variables|Default|GetSkeletalMesh))
  ;[1 1 1] Skin personaje
  (bind _asbp_third_person_character (Utilities|Casting|CastToBP_ThirdPersonCharacter (Game|GetPlayerCharacter 0)))
  (bind _output_get (Variables|Default|SetposicionInicial (Transformation|GetActorLocation)))
  (Variables|Default|SetdireccionNPCs (< (.x _output_get) (.x (Transformation|GetActorLocation _asbp_third_person_character))))
  (if (Variables|/Game/ThirdPerson/Blueprints/BP_ThirdPersonCharacter.BP_ThirdPersonCharacter_C|GetesTutorial _asbp_third_person_character)
    _
    (else
      (CallFunction|Movimiento)))
  (Utilities|FlowControl|Sequence
    (:then_0
      (switch int (Math|Random|RandomIntegerinRange 0 2)
        (:0
          (Variables|Default|Settipo%20personaje "NewEnumerator0")
          (Components|SkeletalMesh|SetSkeletalMeshAsset _skeletalmesh "/Game/Personajes/SetaPj/Walking.Walking")
          (Components|Animation|PlayAnimation _skeletalmesh "/Game/Personajes/SetaPj/Walking_Anim_mixamo_com.Walking_Anim_mixamo_com" true))
        (:1
          (Variables|Default|Settipo%20personaje "NewEnumerator1")
          (Components|SkeletalMesh|SetSkeletalMeshAsset _skeletalmesh "/Game/Characters/Mannequins/Meshes/SKM_Manny.SKM_Manny")
          (Components|Animation|PlayAnimation _skeletalmesh "/Game/Characters/Mannequins/Animations/Manny/MM_Walk_Fwd.MM_Walk_Fwd" true))
        (:2
          (Variables|Default|Settipo%20personaje "NewEnumerator2")
          (Components|SkeletalMesh|SetSkeletalMeshAsset _skeletalmesh "/Game/Characters/Mannequin_UE4/Meshes/SK_Mannequin.SK_Mannequin")
          (Components|Animation|PlayAnimation _skeletalmesh "/Game/Characters/Mannequins/Animations/Manny/MM_Walk_Fwd.MM_Walk_Fwd" true))))
    (:then_1
      ;[1 1 1] Texto diálogo
      (bind _asw_dialogo (Utilities|Casting|CastTow_dialogo (UserInterface|GetWidget (Variables|Default|Getdialogo))))
      (bind _output_get_2 (Variables|/Game/w_dialogo.w_dialogo_C|SetDialogo _asw_dialogo (.OutItem (Utilities|Array|Random (Variables|Default|GetFrases)))))
      (bind _asw_dialogo_2 (Utilities|Casting|CastTow_dialogo (UserInterface|GetWidget (Variables|Default|Getdialogo1))))
      (Variables|/Game/w_dialogo.w_dialogo_C|SetDialogo _asw_dialogo_2 _output_get_2))))

(fn ConstructionScript)